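; BP_PlayerShip is a clickable player ship that can be selected in the game.
; On begin play it caches the PlayerPawn and gives its UI_PlayerShip widget a reference to itself.
; Clicking its Sphere calls SelectShip, stores the ship as the pawn's SelectedShip and fires the pawn's select-ship event dispatcher.
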(event `self.ReceiveBeginPlay`
  (bind _asplayer_pawn (cast `/Game/Blueprints/PlayerPawn` (`GameplayStatics.GetPlayerPawn` 0)))
  (set `self.As Player Pawn` _asplayer_pawn)
  (bind _asui_player_ship (cast `/Game/UserInterface/UI_PlayerShip` (`WidgetComponent.GetWidget` (`self.Widget`))))
  (set `/Game/UserInterface/UI_PlayerShip.Ship` self _asui_player_ship))

(event `self.Sphere.OnClicked`
  (params (TouchedComponent :type "PrimitiveComponent Object Reference") (ButtonPressed :type "Key Structure"))
  (bind _as_player_pawn (`self.As Player Pawn`))
  (`self.SelectShip`)
  (set `/Game/Blueprints/PlayerPawn.SelectedShip` self _as_player_pawn)
  (`/Game/Blueprints/PlayerPawn.SelectShipEventDispatcher` _as_player_pawn))

(fn `UserConstructionScript`)