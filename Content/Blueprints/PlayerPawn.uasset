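; PlayerPawn is the player's pawn, which sets up the game control UI for a board game with selectable ships.
; On BeginPlay it creates the UI_GameControl widget, adds it to the viewport and hands it the first BP_Board found in the level.
; It also binds to the SelectShip event dispatcher, copying its SelectedShip into the widget whenever that fires.
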(event `self.ReceiveBeginPlay`
  (`|ExecutionSequence`
    (:`then_0`
      (bind _returnvalue (`|CreateWidget` "/Game/UserInterface/UI_GameControl.UI_GameControl_C"))
      (bind _output_get (set `self.ControlWidget` _returnvalue))
      (`UserWidget.AddToViewport` _output_get 0)
      (bind _outactors (`GameplayStatics.GetAllActorsOfClass` "/Game/Blueprints/World/BP_Board.BP_Board_C"))
      (set `/Game/UserInterface/UI_GameControl.Board` (`|GetArrayItem` _outactors) (`self.ControlWidget`)))
    (:`then_1`
      (add `self.SelectShipEventDispatcher` (delegate `SetSelectedShip`)))))

(event `SetSelectedShip`
  (set `/Game/UserInterface/UI_GameControl.SelectedShip` (`self.SelectedShip`) (`self.ControlWidget`)))

(fn `UserConstructionScript`)