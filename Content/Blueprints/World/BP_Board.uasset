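; Board Blueprint for a tile-based ship game that syncs player and opponent ship state with a local HTTP server through VaRest.
; BeginPlay requests a new game, prepares six reusable JSON ship objects and binds EndMove.
; EndMove posts all ships to update_map, refreshes stats and highlights the selected ship's neighboring tiles.
; The update callback fetches actions, but their handling and the new-game response are empty stubs.
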(event `self.ReceiveBeginPlay`
  (bind _returnvalue (subsystem `VaRestSubsystem`))
  (`|ExecutionSequence`
    (:`then_0`
      (add `self.EndMoveEventDispatcher` (delegate `EndMove`))
      (`VaRestSubsystem.CallURL` (subsystem `VaRestSubsystem`) "localhost:8000/new_game" "GET" "json" null (delegate `NewGame`))
      (`|ExecutionSequence`
        (:`then_0`
          (bind _returnvalue_2 (`VaRestSubsystem.ConstructVaRestJsonObject` _returnvalue))
          (set `self.JsonObject` _returnvalue_2))
        (:`then_1`
          (for _ (range 6)
            (bind _returnvalue_3 (`VaRestSubsystem.ConstructVaRestJsonObject` _returnvalue))
            (`KismetArrayLibrary.Array_Add` (`self.ShipState`) _returnvalue_3)))))
    (:`then_1`
      (bind _asplayer_pawn (cast `/Game/Blueprints/PlayerPawn` (`GameplayStatics.GetPlayerPawn` 0)))
      (set `self.Control Widget` (`/Game/Blueprints/PlayerPawn.ControlWidget` _asplayer_pawn)))))

(event `NewGame`
  (params (Request :type "VaRestRequestJSON Object Reference")))

(event `EndMove`
  (`|ExecutionSequence`
    (:`then_0`
      (`|ExecutionSequence`
        (:`then_0`
          (for (_array_element _array_index) (`self.SpawnedPlayerShips`)
            (bind _returnvalue (`CPP_PlayerShip.CreateJsonData` _array_element))
            (bind _output (`|GetArrayItem` (`self.ShipState`) _array_index))
            (`VaRestJsonObject.SetMapFields_int32` _output _returnvalue)
            (`VaRestJsonObject.SetObjectField` (`self.JsonObject`) (`KismetStringLibrary.Conv_IntToString` (+ _array_index 1)) _output)))
        (:`then_1`
          (for (_array_element_2 _array_index_2) (`self.SpawnedOpponentShips`)
            (bind _returnvalue_2 (`CPP_OpponentShip.CreateJsonData` _array_element_2))
            (bind _output_2 (`|GetArrayItem` (`self.ShipState`) (+ _array_index_2 3)))
            (`VaRestJsonObject.SetMapFields_int32` _output_2 _returnvalue_2)
            (`VaRestJsonObject.SetObjectField` (`self.JsonObject`) (`KismetStringLibrary.Conv_IntToString` (+ _array_index_2 4)) _output_2)))
        (:`then_2`
          (`VaRestSubsystem.CallURL` (subsystem `VaRestSubsystem`) "localhost:8000/update_map" "POST" "json" (`self.JsonObject`) (delegate `UpdateMap`)))))
    (:`then_1`
      (`self.UpdateShipStats`)
      (`CPP_TileToSpawn.HighlightNeighbors` (`CPP_PlayerShip.Tile` (`self.SelectedShip`))))))

(event `UpdateMap`
  (params (Request :type "VaRestRequestJSON Object Reference"))
  (`VaRestSubsystem.CallURL` (subsystem `VaRestSubsystem`) "localhost:8000/get_actions" "GET" "json" null (delegate `GetActions`)))

(event `GetActions`
  (params (Request :type "VaRestRequestJSON Object Reference"))
  (for _ (`VaRestJsonObject.GetArrayField` (`VaRestRequestJSON.GetResponseObject` Request) "actions")
    _))

(fn `CreateJsonData`)

(fn `UserConstructionScript`)